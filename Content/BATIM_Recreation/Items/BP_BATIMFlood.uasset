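; BP_BATIMFlood is a rising ink flood for the BATIM recreation that slows the player while they are inside it.
; A custom event, guarded by a DoOnce, plays the Rise timeline to lerp the Ink component between Start and End locations.
; Ink overlap events lower the BP_BATIMPlayer's max walk speed on entry and set it to a fixed faster value on exit.
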(event OnComponentBeginOverlap(Ink)
  (params (OverlappedComponent :type Primitive%20Component%20Object%20Reference) (OtherActor :type Actor%20Object%20Reference) (OtherComp :type Primitive%20Component%20Object%20Reference) (OtherBodyIndex :type Integer) (bFromSweep :type Boolean) (SweepResult :type Hit%20Result%20Structure%20%28by%20ref%29))
  ;[0.15 0.15 0.15 0.5] Slow Player down
  (if (== OtherActor (Game|GetPlayerCharacter 0))
    (bind _returnvalue (Actor|GetActorOfClass "/Game/BATIM_Recreation/BP_BATIMPlayer.BP_BATIMPlayer_C"))
    (Variables|/Script/Engine.CharacterMovementComponent|SetMaxWalkSpeed (Variables|/Script/Engine.Character|GetCharacterMovement _returnvalue) 3.5e+02)))

(event OnComponentEndOverlap(Ink)
  (params (OverlappedComponent :type Primitive%20Component%20Object%20Reference) (OtherActor :type Actor%20Object%20Reference) (OtherComp :type Primitive%20Component%20Object%20Reference) (OtherBodyIndex :type Integer))
  ;[0.15 0.15 0.15 0.5] Slow Player down
  (if (== OtherActor (Game|GetPlayerCharacter 0))
    (bind _returnvalue (Actor|GetActorOfClass "/Game/BATIM_Recreation/BP_BATIMPlayer.BP_BATIMPlayer_C"))
    (Variables|/Script/Engine.CharacterMovementComponent|SetMaxWalkSpeed (Variables|/Script/Engine.Character|GetCharacterMovement _returnvalue) 6e+02)))

(event EventFunction
  ;[0.15 0.15 0.15 0.5] Rise
  (Utilities|FlowControl|DoOnce false
    (:Completed
      (bind _up (Timeline|Rise PlayFromStart)
        (:Update
          (Transformation|SetWorldLocation (Variables|Default|GetInk) (Math|Vector|Lerp(Vector) (Variables|Default|GetStart) (Variables|Default|GetEnd) _up) false false))))))

(fn ConstructionScript)