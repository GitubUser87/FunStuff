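; BP_BATIMValve is an interactable valve item that turns once and then notifies other actors.
; Interact works only after the Function event enables it, and a DoOnce limits it to a single use.
; A timeline adds relative rotation to the valve mesh each update.
; When it finishes, every actor tagged "Lever" receives a Function message, chaining the valve to those levers.
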(event EventInteract
  ;[0.15 0.15 0.15 0.5] Rotate Valve
  (if (Variables|Default|GetCan?)
    (Utilities|FlowControl|DoOnce false
      (:Completed
        (bind _spin (Timeline|Rotate PlayFromStart)
          (:Update
            (Transformation|AddRelativeRotation (Variables|Default|GetValve) (Math|Rotator|Lerp(Rotator) "0, 0, 0" "1.000000,0.000000,0.000000" _spin) false false))
          (:Finished
            (bind _outactors (Actor|GetAllActorswithTag "Lever"))
            (for _array_element _outactors
              (Class|BPIBatimFunctions|Function(Message) _array_element))))))))

(event EventFunction
  ;[0.15 0.15 0.15 0.5] Enable
  (Variables|Default|SetCan? true))

(fn ConstructionScript)