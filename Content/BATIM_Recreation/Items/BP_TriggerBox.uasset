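; BP_TriggerBox is a one-shot trigger volume that fires tagged actors and shows HUD text when the player enters it.
; The overlap responds only to the player character while Can is true, which the Function event sets, so other actors can arm it.
; A DoOnce then sends FunctionMessage to every actor with Tag and passes Main and Hint text to the BP_BATIMHud widget.
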(event OnComponentBeginOverlap(Trigger)
  (params (OverlappedComponent :type Primitive%20Component%20Object%20Reference) (OtherActor :type Actor%20Object%20Reference) (OtherComp :type Primitive%20Component%20Object%20Reference) (OtherBodyIndex :type Integer) (bFromSweep :type Boolean) (SweepResult :type Hit%20Result%20Structure%20%28by%20ref%29))
  ;[0.15 0.15 0.15 0.5] Trigger Functions
  (if (and (== OtherActor (Game|GetPlayerCharacter 0)) (Variables|Default|GetCan?))
    (Utilities|FlowControl|DoOnce false
      (:Completed
        (bind _outactors (Actor|GetAllActorswithTag (Variables|Default|GetTag)))
        (for _array_element _outactors
          (Class|BPIBatimFunctions|Function(Message) _array_element))
        (bind _foundwidgets (Widget|GetAllWidgetsOfClass "/Game/BATIM_Recreation/BP_BATIMHud.BP_BATIMHud_C" false))
        (Class|BPIBatimFunctions|SetText(Message) (Utilities|Array|Get(acopy) _foundwidgets) (Variables|Default|GetMain) (Variables|Default|GetHint))))))

(event EventFunction
  ;[0.15 0.15 0.15 0.5] Trigger Functions
  (Variables|Default|SetCan? true))

(fn ConstructionScript)