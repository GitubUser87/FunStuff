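; BP_BATIMLever is a lever in the BATIM recreation that stays locked until it has been activated six times.
; Each Function call increments a counter; at six it shows main and hint text on BP_BATIMHud and allows pulling.
; Interact then plays the Pull timeline from the start, lerping the lever's relative rotation.
; When the timeline finishes, it calls FunctionMessage on its Trigger reference.
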(event EventInteract
  ;[0.15 0.15 0.15 0.5] Pull
  (if (Variables|Default|GetCan?)
    (bind _pulllever (Timeline|Pull PlayFromStart)
      (:Update
        (Transformation|SetRelativeRotation (Variables|Default|GetLever) (Math|Rotator|Lerp(Rotator) "0.000000,0.000000,30.000000" "0.000000,0.000000,130.000000" _pulllever) false false))
      (:Finished
        (Class|BPIBatimFunctions|Function(Message) (Variables|Default|GetTrigger))))))

(event EventFunction
  ;[0.15 0.15 0.15 0.5] Activate
  (bind _output_get (Variables|Default|SetAmount (+ (Variables|Default|GetAmount) 1)))
  (if (== _output_get 6)
    (bind _foundwidgets (Widget|GetAllWidgetsOfClass "/Game/BATIM_Recreation/BP_BATIMHud.BP_BATIMHud_C" false))
    (Class|BPIBatimFunctions|SetText(Message) (Utilities|Array|Get(acopy) _foundwidgets) (Variables|Default|GetMain) (Variables|Default|GetHint))
    (Variables|Default|SetCan? true)))

(fn ConstructionScript)