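; BP_BATIMItem is a collectible pickup in a BATIM recreation that the player can take into their item list.
; On BeginPlay it looks up its row in the ItemData table and applies that row's mesh.
; A separate event enables pickup via the Can flag.
; When interacted with while enabled, it adds the mesh uniquely to BP_BATIMPlayer's ItemArray and destroys itself.
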(event EventBeginPlay
  ;[0.15 0.15 0.15 0.5] Set Item Data
  (bind _returnvalue (Utilities|GetDataTableRow (Variables|Default|GetItemData) (.rowname (Variables|Default|GetDataRow)))
    (:then
      (Components|StaticMesh|SetStaticMesh (Variables|Default|GetItem) (.ItemMesh (Utilities|Struct|BreakBATIM_Items _returnvalue))))))

(event EventFunction
  ;[0.15 0.15 0.15 0.5] Can?
  (Variables|Default|SetCan? true))

(event EventInteract
  ;[0.15 0.15 0.15 0.5] Interact
  (if (Variables|Default|GetCan?)
    (bind _returnvalue (Actor|GetActorOfClass "/Game/BATIM_Recreation/BP_BATIMPlayer.BP_BATIMPlayer_C"))
    (bind _output_get (Variables|Default|SetPlayerRef _returnvalue))
    (Utilities|Array|AddUnique (Variables|/Game/BATIM_Recreation/BP_BATIMPlayer.BP_BATIMPlayer_C|GetItemArray _output_get) (.ItemMesh (Utilities|Struct|BreakBATIM_Items (stale EventBeginPlay _returnvalue))))
    (Actor|DestroyActor)))

(fn ConstructionScript)