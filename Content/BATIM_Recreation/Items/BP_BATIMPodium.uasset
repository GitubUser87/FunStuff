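; BP_BATIMPodium is an interactable podium for the BATIM recreation that accepts a specific item from the player's inventory.
; On interact, it looks up its ItemData row and searches BP_BATIMPlayer's ItemArray for the matching mesh.
; A match is displayed on the podium, removed from the inventory and sets Activate.
; Once activated, it calls FunctionMessage a single time on every actor with its configured Tag, triggering linked actors.
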(event EventInteract
  (bind _returnvalue (Utilities|GetDataTableRow (Variables|Default|GetItemData) (.rowname (Variables|Default|GetDataRow)))
    (:then
      (bind _array_element (Utilities|Array|ForEachLoopwithBreak (Variables|/Game/BATIM_Recreation/BP_BATIMPlayer.BP_BATIMPlayer_C|GetItemArray (Variables|Default|GetBATIMPlayerRef)) :!label _label)
        (:LoopBody
          (if (== _array_element (.ItemMesh (Utilities|Struct|BreakBATIM_Items _returnvalue)))
            (Components|StaticMesh|SetStaticMesh (Variables|Default|GetItem) _array_element)
            (Variables|Default|SetActivate? true)
            (Utilities|Array|RemoveItem (Variables|/Game/BATIM_Recreation/BP_BATIMPlayer.BP_BATIMPlayer_C|GetItemArray (Variables|Default|GetBATIMPlayerRef)) _array_element)
            (goto _label Break)))
        (:Completed
          (if (Variables|Default|GetActivate?)
            (Utilities|FlowControl|DoOnce false
              (:Completed
                (bind _outactors (Actor|GetAllActorswithTag (Variables|Default|GetTag)))
                (for _array_element_2 _outactors
                  (Class|BPIBatimFunctions|Function(Message) _array_element_2))))))))))

(event EventBeginPlay
  ;[0.15 0.15 0.15 0.5] PlayuerRef
  (bind _returnvalue (Actor|GetActorOfClass "/Game/BATIM_Recreation/BP_BATIMPlayer.BP_BATIMPlayer_C"))
  (Variables|Default|SetBATIMPlayerRef _returnvalue))

(fn ConstructionScript)

(fn Function)